(event Input|EnhancedActionEvents|EnhancedInputActionIA_Build
  (params (ActionValue :type Boolean) (ElapsedSeconds :type Float%20%28double-precision%29) (TriggeredSeconds :type Float%20%28double-precision%29) (InputAction :type Input%20Action%20Object%20Reference :default "/Game/Input/IA_Build.IA_Build"))
  (bind _hud (Variables|Default|GetHUD))
  (:Started
    (if (not (Variables|Default|GetToggleBuffer))
      (Variables|/Game/GUI/WBP_HUD.WBP_HUD_C|SetToggleBuffer _hud true)
      (Default|ToggleBuildMenu _hud true)))
  (:Completed
    (Variables|Default|SetToggleBuffer false)))

(event EventBeginPlay
  (bind _returnvalue (PlayerController|LocalPlayerSubsystems|GetEnhancedInputLocalPlayerSubsystem))
  (bind _self self)
  (Utilities|FlowControl|Sequence
    (:then_0
      (Utilities|IsValid _returnvalue
        (:Is%20Valid
          (Input|AddMappingContext _returnvalue "/Game/Input/IMC_Main.IMC_Main" 0 "(bIgnoreAllPressedKeysUntilRelease=True,bForceImmediately=False,bNotifyUserSettings=False)"))))
    (:then_1
      (bind _returnvalue_2 (UserInterface|CreateWidget "/Game/GUI/WBP_HUD.WBP_HUD_C" _self _self))
      (UserInterface|Viewport|AddtoViewport _returnvalue_2 0)
      (Variables|Default|SetHUD _returnvalue_2))
    (:then_2
      (bind _asbp_player_character (Utilities|Casting|CastToBP_PlayerCharacter (Game|Player|GetPlayerPawn 0)))
      (Variables|Default|SetPlrCharacter _asbp_player_character))))

(fn ConstructionScript)